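; Cinematic camera child actor that travels along a spline when possessed, serving paintings, the ending or other scripted shots.
; Possession binds a Tick-driven travel event that moves the view by spline time without rotating it, and unlocks linked interactables after a delay.
; One second before travel ends, a DoOnce returns to the interaction camera, revealing painting dialog first, or shows the end-game widget.
; Painting cameras register with the game instance on BeginPlay.
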(event `self.ReceiveBeginPlay`
  (`parent.ReceiveBeginPlay`)
  (if (`self.ForPainting`)
    (bind _asadventure_game_istance (cast `/Game/Config/GameInstance/AdventureGameIstance` (`GameplayStatics.GetGameInstance`)))
    (`/Game/Config/GameInstance/AdventureGameIstance.SetUpPaintingCamera` _asadventure_game_istance (`self.ReferenceIndex`) self)))

(event `self.ReceiveTick`
  (params (DeltaSeconds :type "Float (single-precision)"))
  (`self.CameraTreaveling` DeltaSeconds))

(event `self.OnPossess`
  (bind _as_adventure_game_istance (`self.As Adventure Game Istance`))
  (set `self.CurrentTime` 0.0)
  (add `self.CameraTreaveling` (delegate `CameraTreaveling_Event`))
  (`KismetSystemLibrary.Delay` (`self.DelayBeforeInteract`))
  (for _array_element (`self.UnlockInteraction`)
    (message `/Game/BlueprintActors/InteractibleObjects/BPI_Interact.UnlockInteract` _array_element (0.0 0.0 0.0) 0))
  (goto _label :!via `Reset`))

(event `CameraTreaveling_Event` :!signature `self.CameraTreaveling`
  (params (WorldDelataSeconds :type "Float (double-precision)"))
  (bind _as_adventure_game_istance (`self.As Adventure Game Istance`))
  (bind _output_get (set `self.CurrentTime` (+ WorldDelataSeconds (`self.CurrentTime`))))
  (`SceneComponent.K2_SetWorldLocation` (`self.CameraView`) (`SplineComponent.GetLocationAtTime` (`self.CameraTravelSpline`) (/ _output_get (`self.TimeToTravel`)) "World" false) false false)
  (if (<= (- (`self.TimeToTravel`) 1.0) (`self.CurrentTime`))
    (`/Engine/EditorBlueprintResources/StandardMacros.DoOnce` false :!label _label
      (:`Completed`
        (if (`self.ForPainting`)
          (`/Game/Config/GameInstance/AdventureGameIstance.RevealPaintingSentenceDialog` _as_adventure_game_istance)
          (`/Game/Config/GameInstance/AdventureGameIstance.BackInteractionCamera` _as_adventure_game_istance "NewEnumerator1" :!label _label_2)
          (elif (`self.IsEndingCamera`)
            (bind _returnvalue (`|CreateWidget` "/Game/UserInterface/W_EndGame.W_EndGame_C"))
            (`UserWidget.AddToViewport` _returnvalue 0)
            (else
              (goto _label_2))))))))

(fn `UserConstructionScript`
  (`parent.UserConstructionScript`))