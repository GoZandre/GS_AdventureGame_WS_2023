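; Interactable music box handle in the Cabaret set that spins on its own, either from BeginPlay or once interacted with.
; HandleTimeline drives HandleRotation through a full turn, with its play rate held at zero when StartOn is false.
; StartInteract runs a second timeline that ramps that play rate from zero to PlayRate for a gradual spin-up.
; Mouse-deprojection and arrow-comparison helpers for manual rotation are present but unused.
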(event `/Game/BlueprintActors/InteractibleObjects/BPI_Interact.StartInteract`
  (params (ImpactLocation :type "Vector Structure") (CollidedComponent :type "ActorComponent Object Reference"))
  (bind _playrate (`self.PlayRate`))
  (bind _handletimeline (`self.HandleTimeline`))
  (bind (_direction _lerp) (`Timeline|PRTimenline` :!via `PlayFromStart`)
    (:`Update`
      (`TimelineComponent.SetPlayRate` _handletimeline (`KismetMathLibrary.Lerp` 0.0 _playrate _lerp)))
    (:`Finished`
      (`TimelineComponent.SetPlayRate` _handletimeline _playrate))))

(event `self.ReceiveBeginPlay`
  (bind _handletimeline (`self.HandleTimeline`))
  (`TimelineComponent.SetPlayRate` _handletimeline (`self.PlayRate`))
  (if (`self.StartOn`)
    (bind (_direction _lerp) (`Timeline|HandleTimeline` :!label _label)
      (:`Update`
        (`SceneComponent.K2_SetRelativeRotation` (`self.HandleRotation`) (`KismetMathLibrary.RLerp` (struct) (struct :`Roll` 360.0) _lerp) false false)))
    (else
      (`TimelineComponent.SetPlayRate` _handletimeline 0.0)
      (goto _label))))

(fn `UserConstructionScript`
  (`parent.UserConstructionScript`))