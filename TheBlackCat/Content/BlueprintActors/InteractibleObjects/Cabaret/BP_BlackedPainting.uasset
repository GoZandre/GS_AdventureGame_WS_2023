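; BP_BlackedPainting is an interactible cabaret painting that reveals itself and presents an item when unlocked.
; On unlock, it spawns the actor class from the LinkedItem data table row and attaches it to an arrow component.
; Two half-speed timelines then run together: one animates a radius parameter on the frame mesh's dynamic material, the other lerps the arrow, carrying the item, toward its final position.
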(event `self.ReceiveBeginPlay`
  (`parent.ReceiveBeginPlay`)
  (bind _returnvalue (`PrimitiveComponent.CreateDynamicMaterialInstance` (`self.SM_Cadres_SM_Cadre_01`) 1 (`self.SourceMaterial`) "None"))
  (set `self.MaterialInstance` _returnvalue)
  (`TimelineComponent.SetPlayRate` (`self.RevealTimeline`) 0.5)
  (`TimelineComponent.SetPlayRate` (`self.ObjectLocationLerp`) 0.5))

(event `/Game/BlueprintActors/InteractibleObjects/BPI_Interact.UnlockInteract`
  (params (ImpactLocation :type "Vector Structure") (UnlockIndex :type Integer))
  (bind _spawnitemarrow (`self.SpawnItemArrow`))
  (bind (_datatable _rowname) (break `DataTableRowHandle` (`self.LinkedItem`)))
  (`parent.UnlockInteract` ImpactLocation UnlockIndex)
  (bind _returnvalue (`|GetDataTableRow` _datatable _rowname)
    (:`then`
      (bind _returnvalue_2 (`|SpawnActorFromClass` (`.ItemActor_22_E6E61AA447787B6299298281A95A7995` (break `/Game/Config/Inventory/S_Item` _returnvalue)) (`SceneComponent.K2_GetComponentToWorld` (`self.SpawnItemArrow`)) "Undefined" "OverrideRootScale" null (`self.LinkedItem`) null))
      (`self.K2_AttachToComponent` _returnvalue_2 (`self.SpawnItemArrow`) "None" "SnapToTarget" "SnapToTarget" "SnapToTarget" true)
      (`|ExecutionSequence`
        (:`then_0`
          (bind (_direction _lerp) (`Timeline|RevealTimeline` :!via `PlayFromStart`)
            (:`Update`
              (`MaterialInstanceDynamic.SetScalarParameterValue` (`self.MaterialInstance`) "RadiusParam" (`KismetMathLibrary.Lerp` -1.0 2.0 _lerp)))))
        (:`then_1`
          (bind (_direction_2 _lerp_2) (`Timeline|ObjectLocationLerp` :!via `PlayFromStart`)
            (:`Update`
              (`SceneComponent.K2_SetRelativeLocation` _spawnitemarrow (`KismetMathLibrary.VLerp` (`SceneComponent.RelativeLocation` _spawnitemarrow) (`SceneComponent.RelativeLocation` (`self.FinalItemPosition`)) _lerp_2) false false))))))))

(fn `UserConstructionScript`
  (`parent.UserConstructionScript`))