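; BP_Interactible is a base actor for interactible puzzle objects, with empty PuzzleSolved, PuzzleUnsloved and CantInteractFeedback events as hooks for children.
; StartInteract enables tick if CanInteract is set, otherwise triggers feedback; UnlockInteract sets that flag.
; While ticking, VerifyCondition calls the solved or unsolved hook from PuzzleCompleted, until EndInteract, also run at BeginPlay, disables tick.
; A helper finds the component nearest a world impact location.
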(event `self.ReceiveBeginPlay`
  (`/Game/BlueprintActors/InteractibleObjects/BPI_Interact.EndInteract`))

(event `/Game/BlueprintActors/InteractibleObjects/BPI_Interact.StartInteract`
  (params (ImpactLocation :type "Vector Structure"))
  (if (`self.CanInteract`)
    (`self.SetActorTickEnabled` true)
    (else
      (`self.CantInteractFeedback`))))

(event `/Game/BlueprintActors/InteractibleObjects/BPI_Interact.UnlockInteract`
  (set `self.CanInteract` true))

(event `/Game/BlueprintActors/InteractibleObjects/BPI_Interact.EndInteract`
  (`self.SetActorTickEnabled` false))

(event `CantInteractFeedback`)

(event `self.ReceiveTick`
  (params (DeltaSeconds :type "Float (single-precision)"))
  (`self.VerifyCondition`))

(event `VerifyCondition`
  (if (`self.PuzzleCompleted`)
    (`self.PuzzleSolved`)
    (else
      (`self.PuzzleUnsloved`))))

(event `PuzzleSolved`
  ;[1 1 1] Inherit functions
)

(event `PuzzleUnsloved`
  ;[1 1 1] Inherit functions
)

(fn `GetNearestComponent`
  (params (WorldImpactLocation :type "Vector Structure") (ObjectsToCompare :type "Array of StaticMeshComponent Object Reference"))
  (locals (LocalNearestComponent :type Integer) (LocalNearestDistance :type "Float (double-precision)"))
  (set `local.LocalNearestDistance` 1000000000000.0)
  (for (_array_element _array_index) ObjectsToCompare
    (bind _returnvalue (`KismetMathLibrary.VSize` (- (`SceneComponent.K2_GetComponentLocation` _array_element) WorldImpactLocation)))
    (if (< _returnvalue (`local.LocalNearestDistance`))
      (set `local.LocalNearestComponent` _array_index)
      (set `local.LocalNearestDistance` _returnvalue)))
  (set `self.NearestComponent` (`|GetArrayItem` ObjectsToCompare (`local.LocalNearestComponent`)))
  (return))

(fn `UserConstructionScript`)