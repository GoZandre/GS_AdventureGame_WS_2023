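; Cat figure puzzle in which the player turns three rotators with the mouse to reach solution angles.
; Interaction selects the rotator nearest the impact point and stores a yaw offset.
; Tick interpolates that rotator toward the deprojected cursor's yaw, snapped to a grid.
; VerifyCondition requires all three yaw checks within a margin, though rotators 2 and 3 take their upper bound from zero; solving prints "Win".
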(event `self.ReceiveBeginPlay`
  ;[1 1 1] BaseFunction
  (`parent.ReceiveBeginPlay`))

(event `self.VerifyCondition`
  ;[1 1 1] BaseFunction
  (`parent.VerifyCondition`)
  (set `self.PuzzleCompleted` (and (`self.PuzzleCondition_Rotator1`) (`self.PuzzleCondition_Rotator2`) (`self.PuzzleCondition_Rotator3`))))

(event `self.PuzzleSolved`
  ;[1 1 1] BaseFunction
  (`parent.PuzzleSolved`)
  (`KismetSystemLibrary.PrintString` "Win"))

(event `self.PuzzleUnsloved`
  ;[1 1 1] BaseFunction
  (`parent.PuzzleUnsloved`))

(event `/Game/BlueprintActors/InteractibleObjects/BPI_Interact.StartInteract`
  (params (ImpactLocation :type "Vector Structure") (CollidedComponent :type "ActorComponent Object Reference"))
  ;[1 1 1] BaseFunction
  (`self.GetNearestComponent` ImpactLocation (`|MakeArray` (`self.Rotator_01`) (`self.Rotator_02`) (`self.Rotator_03`)))
  (set `self.BaseRotator` (`self.GetBaseRotation`))
  (`parent.StartInteract` ImpactLocation null))

(event `self.ReceiveTick`
  (params (DeltaSeconds :type "Float (single-precision)"))
  (bind _nearestcomponent (`self.NearestComponent`))
  (bind (_worldlocation _worlddirection) (`PlayerController.DeprojectMousePositionToWorld` (`GameplayStatics.GetPlayerController` 0)))
  (bind _returnvalue (`SceneComponent.K2_GetComponentLocation` _nearestcomponent))
  (bind (_returnvalue_roll _returnvalue_pitch _returnvalue_yaw) (`KismetMathLibrary.BreakRotator` (`KismetMathLibrary.FindLookAtRotation` _returnvalue (+ _worldlocation (* _worlddirection (- (`KismetMathLibrary.VSize` (- _returnvalue _worldlocation)) 10.0))))))
  (`parent.ReceiveTick` DeltaSeconds)
  (`SceneComponent.K2_SetRelativeRotation` _nearestcomponent (`KismetMathLibrary.RInterpTo` (`SceneComponent.RelativeRotation` _nearestcomponent) (`KismetMathLibrary.MakeRotator` 0.0 0.0 (`KismetMathLibrary.GridSnap_Float` (- _returnvalue_yaw (`self.BaseRotator`)) (`self.RotationGrid`))) DeltaSeconds 10.0) false false))

(fn `UserConstructionScript`
  (`parent.UserConstructionScript`))