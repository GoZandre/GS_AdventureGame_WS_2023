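; Inventory camera pawn that presents an item for close inspection and lets the player rotate it with look input.
; Taken items lerp by timeline to an inspection component, which smoothly follows a pitch-clamped objective rotation.
; SwitchItem spawns a replacement in place; Back lerps the item away, destroys it and asks the game instance to return to the previous camera.
; The camera optionally destroys itself when the last camera exits.
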(event `self.OnPossess`
  ;[1 1 1] Init
  (`TimelineComponent.SetPlayRate` (`self.LerpTransform`) (`self.GetItemSpeed`))
  (`TimelineComponent.SetPlayRate` (`self.PutItemAwayLerp`) (`self.PutAwayItemSpeed`)))

(event `TakeItem`
  (params (Item :type "/Game/BlueprintActors/Items/BP_Item Object Reference") (ItemSize :type "Vector Structure"))
  (bind _itemactor (`self.ItemActor`))
  ;[1 1 1] Init
  (`SceneComponent.SetRelativeScale3D` (`self.ItemInspection`) ItemSize)
  (bind _output_get (set `self.ItemActor` Item))
  (`self.K2_AttachToComponent` _output_get (`self.ItemInspection`) "None" "KeepWorld" "KeepWorld" "KeepWorld" true)
  (bind (_direction _lerpvalue) (`Timeline|LerpTransform` :!via `PlayFromStart`)
    (:`Update`
      (`self.K2_SetActorTransform` _itemactor (`KismetMathLibrary.TLerp` (`self.GetTransform` _itemactor) (`SceneComponent.K2_GetComponentToWorld` (`self.ItemInspection`)) _lerpvalue) false false))
    (:`Finished`
      (add `self.LookRotation` (delegate `LookAround`)))))

(event `LookAround` :!signature `self.LookRotation`
  (params (ActionValue :type "Vector2D Structure"))
  (bind (_x _y) (`KismetMathLibrary.BreakVector2D` ActionValue))
  (bind _inspectionobjective (`self.InspectionObjective`))
  (bind _sensibility (`self.Sensibility`))
  (bind (_relativerotation_roll _relativerotation_pitch _relativerotation_yaw) (`KismetMathLibrary.BreakRotator` (`SceneComponent.RelativeRotation` _inspectionobjective)))
  ;[1 1 1] Init
  (`SceneComponent.K2_AddRelativeRotation` _inspectionobjective (`KismetMathLibrary.MakeRotator` 0.0 (* _y _sensibility) (* _x _sensibility -1.0)) false false)
  (`SceneComponent.K2_SetRelativeRotation` _inspectionobjective (`KismetMathLibrary.MakeRotator` _relativerotation_roll (`KismetMathLibrary.ClampAngle` _relativerotation_pitch -60.0 60.0) _relativerotation_yaw) false false))

(event `EnhancedInput|/Game/Config/Input/Actions/IA_Look`
  (params (ActionValue :type "Vector2D Structure") (ElapsedSeconds :type "Float (double-precision)") (TriggeredSeconds :type "Float (double-precision)") (InputAction :type "InputAction Object Reference" :default "/Game/Config/Input/Actions/IA_Look.IA_Look"))
  ;[1 1 1] Init
  (:`Started`
    (`self.LookRotation` ActionValue :!label _label))
  (:`Ongoing`
    (goto _label)))

(event `self.ReceiveTick`
  (params (DeltaSeconds :type "Float (single-precision)"))
  (bind _iteminspection (`self.ItemInspection`))
  ;[1 1 1] Init
  (`SceneComponent.K2_SetRelativeRotation` _iteminspection (`KismetMathLibrary.RInterpTo` (`SceneComponent.RelativeRotation` _iteminspection) (`SceneComponent.RelativeRotation` (`self.InspectionObjective`)) DeltaSeconds 5.0) false false))

(event `self.ReceiveBeginPlay`
  ;[1 1 1] Init
  (`parent.ReceiveBeginPlay`)
  (bind _asadventure_game_istance (cast `/Game/Config/GameInstance/AdventureGameIstance` (`GameplayStatics.GetGameInstance`)))
  (set `self.AdventureInstance` _asadventure_game_istance)
  (if (`self.DestroyOnExit`)
    (add `/Game/Config/GameInstance/AdventureGameIstance.OnExitLastCamera` (`self.AdventureInstance`) (delegate `EventDestroySelf`))))

(event `EventDestroySelf`
  ;[1 1 1] Init
  (`KismetSystemLibrary.PrintString` "Inventory camera destroy")
  (`self.K2_DestroyActor`))

(event `EnhancedInput|/Game/Config/Input/Actions/IA_Back`
  (params (ActionValue :type Boolean) (ElapsedSeconds :type "Float (double-precision)") (TriggeredSeconds :type "Float (double-precision)") (InputAction :type "InputAction Object Reference" :default "/Game/Config/Input/Actions/IA_Back.IA_Back"))
  (bind _itemactor (`self.ItemActor`))
  (:`Triggered`
    (set `PlayerController.bShowMouseCursor` true (`GameplayStatics.GetPlayerController` 0))
    (bind (_direction _lerpvalue) (`Timeline|PutItemAwayLerp` :!via `PlayFromStart`)
      (:`Update`
        (`self.K2_SetActorTransform` _itemactor (`KismetMathLibrary.TLerp` (`self.GetTransform` _itemactor) (`SceneComponent.K2_GetComponentToWorld` (`self.ItemPutAway`)) _lerpvalue) false false))
      (:`Finished`
        (`self.K2_DestroyActor` (`self.ItemActor`))
        (`/Game/Config/GameInstance/AdventureGameIstance.BackInteractionCamera` (`self.As Adventure Game Istance`) (`self.FadeTransition`))))))

(event `SwitchItem`
  (params (NewItem :type "/Game/BlueprintActors/Items/BP_Item Class Reference"))
  (bind _iteminspection (`self.ItemInspection`))
  (`self.K2_DestroyActor` (`self.ItemActor`))
  (bind _returnvalue (`|SpawnActorFromClass` NewItem (`SceneComponent.K2_GetComponentToWorld` _iteminspection) "Undefined" "OverrideRootScale" null null))
  (bind _output_get (set `self.ItemActor` _returnvalue))
  (`self.K2_AttachToComponent` _output_get _iteminspection "None" "KeepWorld" "KeepWorld" "KeepWorld" true))

(fn `UserConstructionScript`
  (`parent.UserConstructionScript`))