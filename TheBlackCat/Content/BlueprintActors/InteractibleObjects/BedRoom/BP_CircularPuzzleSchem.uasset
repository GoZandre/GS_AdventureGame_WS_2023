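; Bedroom circular puzzle interactible where the player rotates rings with the mouse until they match an objective orientation.
; Interaction takes the clicked mesh's attach parent as the ring pivot and stores its angular offset from the mouse.
; Tick eases that pivot's yaw toward the deprojected mouse point, snapped to a rotation grid.
; Completion requires outer and middle arrows within a margin; solving disables interaction and tick.
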(event `self.ReceiveBeginPlay`
  ;[1 1 1] BaseFunction
  (`parent.ReceiveBeginPlay`))

(event `self.VerifyCondition`
  ;[1 1 1] BaseFunction
  (`parent.VerifyCondition`)
  (set `self.PuzzleCompleted` (and (`self.CompareArrow` (`self.OuterRingArrow`)) (`self.CompareArrow` (`self.MiddleRingArrow`)))))

(event `self.PuzzleSolved`
  ;[1 1 1] BaseFunction
  (`parent.PuzzleSolved`)
  (set `self.CanInteract` false)
  (`self.SetActorTickEnabled` false))

(event `self.PuzzleUnsloved`
  ;[1 1 1] BaseFunction
  (`parent.PuzzleUnsloved`))

(event `/Game/BlueprintActors/InteractibleObjects/BPI_Interact.StartInteract`
  (params (ImpactLocation :type "Vector Structure") (CollidedComponent :type "ActorComponent Object Reference"))
  ;[1 1 1] BaseFunction
  (bind _asstatic_mesh_component (cast `StaticMeshComponent` CollidedComponent))
  (set `self.NearestComponent` _asstatic_mesh_component)
  (set `self.CircleParentArrow` (`SceneComponent.GetAttachParent` _asstatic_mesh_component))
  (set `self.BaseRotator` (`self.GetBaseRotation`))
  (`parent.StartInteract` ImpactLocation CollidedComponent))

(event `self.ReceiveTick`
  (params (DeltaSeconds :type "Float (single-precision)"))
  (bind _circleparentarrow (`self.CircleParentArrow`))
  (bind _relativerotation (`SceneComponent.RelativeRotation` _circleparentarrow))
  (`parent.ReceiveTick` DeltaSeconds)
  (`SceneComponent.K2_SetRelativeRotation` _circleparentarrow (`KismetMathLibrary.RInterpTo` _relativerotation (`KismetMathLibrary.MakeRotator` (.roll _relativerotation) (.pitch _relativerotation) (`KismetMathLibrary.GridSnap_Float` (- (.yaw (`KismetMathLibrary.FindLookAtRotation` (`SceneComponent.K2_GetComponentLocation` (`self.CircleParentArrow`)) (`self.GetMouseRot`))) (`self.BaseRotator`)) (`self.RotationGrid`))) DeltaSeconds 10.0) false false))

(fn `UserConstructionScript`
  (`parent.UserConstructionScript`))