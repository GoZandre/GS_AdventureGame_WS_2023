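; Interactible door, filed under debug objects, that swings open and closed and animates when an unlock interaction fires.
; StartInteract alternates through a FlipFlop between open and close timelines, each lerping the DoorRotation component from its current rotation.
; UnlockInteract restarts a separate timeline that drives a slight door swing and turns both handle meshes.
; Both events call their parent implementations first.
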(event `/Game/BlueprintActors/InteractibleObjects/BPI_Interact.StartInteract`
  (params (ImpactLocation :type "Vector Structure") (CollidedComponent :type "ActorComponent Object Reference"))
  (bind _doorrotation (`self.DoorRotation`))
  (bind _doorrotation_2 (`self.DoorRotation`))
  (`parent.StartInteract` ImpactLocation CollidedComponent)
  (`/Engine/EditorBlueprintResources/StandardMacros.FlipFlop`
    (:`A`
      (bind (_direction _lerp) (`Timeline|OpenDoor`)
        (:`Update`
          (`SceneComponent.K2_SetRelativeRotation` _doorrotation_2 (`KismetMathLibrary.RLerp` (`SceneComponent.RelativeRotation` _doorrotation_2) (struct :`Yaw` -90.0) _lerp) false false))))
    (:`B`
      (bind (_direction_2 _lerp_2) (`Timeline|CloseDoor`)
        (:`Update`
          (`SceneComponent.K2_SetRelativeRotation` _doorrotation (`KismetMathLibrary.RLerp` (`SceneComponent.RelativeRotation` _doorrotation) (struct) _lerp_2) false false))))))

(event `/Game/BlueprintActors/InteractibleObjects/BPI_Interact.UnlockInteract`
  (params (ImpactLocation :type "Vector Structure") (UnlockIndex :type Integer))
  (`parent.UnlockInteract` ImpactLocation UnlockIndex)
  (bind (_direction _lerp _lerphandle) (`Timeline|Timeline` :!via `PlayFromStart`)
    (:`Update`
      (`SceneComponent.K2_SetRelativeRotation` (`self.DoorRotation`) (`KismetMathLibrary.RLerp` (struct) (struct :`Yaw` -10.0) _lerp) false false)
      (`SceneComponent.K2_SetRelativeRotation` (`self.SM_DoorHandle_SM_DoorHandle`) (`KismetMathLibrary.RLerp` (struct) (struct :`Pitch` 20.0) _lerphandle) false false)
      (`SceneComponent.K2_SetRelativeRotation` (`self.SM_DoorHandle_SM_DoorHandle1`) (`KismetMathLibrary.RLerp` (struct) (struct :`Pitch` 20.0) _lerphandle) false false))))

(fn `UserConstructionScript`
  (`parent.UserConstructionScript`))