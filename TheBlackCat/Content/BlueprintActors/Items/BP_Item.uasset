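; BP_Item is an interactable item actor that reads its definition from a data table through its ItemsData row handle.
; On StartInteract it sends the row and itself to the Game Instance through AddItemToInventoryMessage.
; Items without CanTakeIt first register their CameraOnLook as an interaction camera on AdventureGameIstance, then send that same message.
; A missing row prints a debug error on screen.
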(event `/Game/BlueprintActors/InteractibleObjects/BPI_Interact.StartInteract`
  (params (ImpactLocation :type "Vector Structure") (CollidedComponent :type "ActorComponent Object Reference"))
  (bind _returnvalue (`GameplayStatics.GetGameInstance`))
  (bind (_datatable _rowname) (break `DataTableRowHandle` (`self.ItemsData`)))
  (bind _returnvalue_2 (`|GetDataTableRow` _datatable _rowname)
    (:`then`
      (if (not (`.CanTakeIt_34_F8B704844128A78A5576F4BEDD5D8BDE` (break `/Game/Config/Inventory/S_Item` _returnvalue_2)))
        (bind _asadventure_game_istance (cast `/Game/Config/GameInstance/AdventureGameIstance` _returnvalue))
        (`/Game/Config/GameInstance/AdventureGameIstance.AddInteractionCamera` _asadventure_game_istance (`self.CameraOnLook`) "NewEnumerator2"))
      (message `/Game/Config/Inventory/BPI_ItemsInteraction.AddItemToInventory` _returnvalue _returnvalue_2 self))
    (:`RowNotFound`
      (`KismetSystemLibrary.PrintString` (`self.DebugError`) true true (struct :`R` 0.567708 :`G` 0.010734 :`A` 1.0)))))

(fn `UserConstructionScript`)