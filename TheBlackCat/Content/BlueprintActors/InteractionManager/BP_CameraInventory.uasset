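; Inventory camera pawn for inspecting an item up close in an adventure game.
; On possess it snaps to the last camera from the game instance; TakeItem attaches the item and lerps it to an inspection point by timeline.
; Once it arrives, look input rotates it through an event dispatcher.
; Back input shows the cursor, lerps the item to a put-away point, destroys it and calls BackInteractionCamera on the game instance.
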(event `self.ReceiveBeginPlay`
  (`parent.ReceiveBeginPlay`))

(event `self.OnPossess`
  ;[1 1 1] Init
  (bind _camera (`/Game/Config/GameInstance/AdventureGameIstance.GetLastCamera` (`self.As Adventure Game Istance`) 1))
  (`self.K2_SetActorTransform` (`self.GetTransform` _camera))
  (`TimelineComponent.SetPlayRate` (`self.LerpTransform`) (`self.GetItemSpeed`))
  (`TimelineComponent.SetPlayRate` (`self.PutItemAwayLerp`) (`self.PutAwayItemSpeed`)))

(event `TakeItem`
  (params (Item :type "/Game/BlueprintActors/Items/BP_Item Object Reference"))
  (bind _itemactor (`self.ItemActor`))
  ;[1 1 1] Init
  (bind _output_get (set `self.ItemActor` Item))
  (`self.K2_AttachToComponent` _output_get (`self.ItemInspection`) "None" "KeepWorld" "KeepWorld" "KeepWorld" true)
  (bind (_direction _lerpvalue) (`Timeline|LerpTransform` :!via `PlayFromStart`)
    (:`Update`
      (`self.K2_SetActorTransform` _itemactor (`KismetMathLibrary.TLerp` (`self.GetTransform` _itemactor) (`SceneComponent.K2_GetComponentToWorld` (`self.ItemInspection`)) _lerpvalue) false false))
    (:`Finished`
      (add `self.LookRotation` (delegate `LookAround`)))))

(event `LookAround` :!signature `self.LookRotation`
  (params (ActionValue :type "Vector2D Structure"))
  (bind (_x _y) (`KismetMathLibrary.BreakVector2D` ActionValue))
  (bind _sensibility (`self.Sensibility`))
  ;[1 1 1] Init
  (`SceneComponent.K2_AddWorldRotation` (`Actor.RootComponent` (`self.ItemActor`)) (`KismetMathLibrary.MakeRotator` (* _y _sensibility) 0.0 (* _x _sensibility -1.0)) false false))

(event `EnhancedInput|/Game/Config/Input/Actions/IA_Look`
  (params (ActionValue :type "Vector2D Structure") (ElapsedSeconds :type "Float (double-precision)") (TriggeredSeconds :type "Float (double-precision)") (InputAction :type "InputAction Object Reference" :default "/Game/Config/Input/Actions/IA_Look.IA_Look"))
  ;[1 1 1] Init
  (:`Started`
    (`self.LookRotation` ActionValue)))

(event `EnhancedInput|/Game/Config/Input/Actions/IA_Back`
  (params (ActionValue :type Boolean) (ElapsedSeconds :type "Float (double-precision)") (TriggeredSeconds :type "Float (double-precision)") (InputAction :type "InputAction Object Reference" :default "/Game/Config/Input/Actions/IA_Back.IA_Back"))
  (bind _itemactor (`self.ItemActor`))
  (:`Triggered`
    (set `PlayerController.bShowMouseCursor` true (`GameplayStatics.GetPlayerController` 0))
    (bind (_direction _lerpvalue) (`Timeline|PutItemAwayLerp` :!via `PlayFromStart`)
      (:`Update`
        (`self.K2_SetActorTransform` _itemactor (`KismetMathLibrary.TLerp` (`self.GetTransform` _itemactor) (`SceneComponent.K2_GetComponentToWorld` (`self.ItemPutAway`)) _lerpvalue) false false))
      (:`Finished`
        (`self.K2_DestroyActor` (`self.ItemActor`))
        (`/Game/Config/GameInstance/AdventureGameIstance.BackInteractionCamera` (`self.As Adventure Game Istance`) false)))))

(fn `UserConstructionScript`
  (`parent.UserConstructionScript`))