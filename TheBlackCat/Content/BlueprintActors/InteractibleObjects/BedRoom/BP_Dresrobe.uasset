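; Bedroom wardrobe interactible with two doors that stays shut until unlocked, built on a parent interaction and puzzle class.
; A failed interaction plays a sped-up timeline that shakes the left door slightly as locked feedback.
; Unlocking waits briefly, then a timeline swings both doors open in opposite directions through rotator lerps.
; Solving the puzzle disables further interaction and actor tick, while the other base events just forward to the parent.
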(event `self.CantInteractFeedback`
  (`TimelineComponent.SetPlayRate` (`self.LockedLerp`) 2.0)
  (bind (_direction _lerpshake) (`Timeline|LockedLerp` :!via `PlayFromStart`)
    (:`Update`
      (`SceneComponent.K2_SetRelativeRotation` (`self.Leftdoor`) (`KismetMathLibrary.RLerp` (struct) (struct :`Yaw` 1.0) _lerpshake) false false))))

(event `self.ReceiveBeginPlay`
  ;[1 1 1] BaseFunction
  (`parent.ReceiveBeginPlay`))

(event `self.VerifyCondition`
  ;[1 1 1] BaseFunction
  (`parent.VerifyCondition`))

(event `self.PuzzleSolved`
  ;[1 1 1] BaseFunction
  (`parent.PuzzleSolved`)
  (set `self.CanInteract` false)
  (`self.SetActorTickEnabled` false))

(event `self.PuzzleUnsloved`
  ;[1 1 1] BaseFunction
  (`parent.PuzzleUnsloved`))

(event `/Game/BlueprintActors/InteractibleObjects/BPI_Interact.StartInteract`
  (params (ImpactLocation :type "Vector Structure") (CollidedComponent :type "ActorComponent Object Reference"))
  ;[1 1 1] BaseFunction
  (`parent.StartInteract` ImpactLocation CollidedComponent))

(event `/Game/BlueprintActors/InteractibleObjects/BPI_Interact.UnlockInteract`
  (params (ImpactLocation :type "Vector Structure") (UnlockIndex :type Integer))
  ;[1 1 1] BaseFunction
  (`parent.UnlockInteract` ImpactLocation UnlockIndex)
  (`KismetSystemLibrary.Delay` 1.0)
  (bind (_direction _lerp) (`Timeline|DresrobeOpen` :!via `PlayFromStart`)
    (:`Update`
      (`SceneComponent.K2_SetRelativeRotation` (`self.Leftdoor`) (`KismetMathLibrary.RLerp` (struct) (struct :`Yaw` 130.0) _lerp) false false)
      (`SceneComponent.K2_SetRelativeRotation` (`self.RightDoor`) (`KismetMathLibrary.RLerp` (struct :`Yaw` 10.0) (struct :`Yaw` -130.0) _lerp) false false))))

(fn `UserConstructionScript`
  (`parent.UserConstructionScript`))