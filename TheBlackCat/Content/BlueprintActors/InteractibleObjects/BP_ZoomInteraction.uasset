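; BP_ZoomInteraction is an interactible object that switches the player to a zoom camera.
; When interaction is allowed, StartInteract disables its CollisionBox and pushes NewCamera through AdventureGameIstance with a transition setting.
; It binds EnableZoomBox to OnExitLastCamera to restore query-only collision.
; UnlockInteract also disables the box and binds that restore event, but adds no camera.
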(event `/Game/BlueprintActors/InteractibleObjects/BPI_Interact.StartInteract`
  (params (ImpactLocation :type "Vector Structure") (CollidedComponent :type "ActorComponent Object Reference"))
  (`parent.StartInteract` ImpactLocation CollidedComponent)
  (`KismetSystemLibrary.PrintString` "Hello")
  (if (`self.CanInteract`)
    (`PrimitiveComponent.SetCollisionEnabled` (`self.CollisionBox`) "NoCollision")
    (bind _asadventure_game_istance (cast `/Game/Config/GameInstance/AdventureGameIstance` (`GameplayStatics.GetGameInstance`)))
    (add `/Game/Config/GameInstance/AdventureGameIstance.OnExitLastCamera` _asadventure_game_istance (delegate `EnableZoomBox`))
    (`/Game/Config/GameInstance/AdventureGameIstance.AddInteractionCamera` _asadventure_game_istance (`self.NewCamera`) "NewEnumerator2")))

(event `EnableZoomBox`
  (`PrimitiveComponent.SetCollisionEnabled` (`self.CollisionBox`) "QueryOnly"))

(event `/Game/BlueprintActors/InteractibleObjects/BPI_Interact.UnlockInteract`
  (params (ImpactLocation :type "Vector Structure") (UnlockIndex :type Integer))
  (`parent.UnlockInteract` ImpactLocation UnlockIndex)
  (`PrimitiveComponent.SetCollisionEnabled` (`self.CollisionBox`) "NoCollision")
  (bind _asadventure_game_istance (cast `/Game/Config/GameInstance/AdventureGameIstance` (`GameplayStatics.GetGameInstance`)))
  (add `/Game/Config/GameInstance/AdventureGameIstance.OnExitLastCamera` _asadventure_game_istance (delegate `EnableZoomBox`)))

(fn `UserConstructionScript`
  (`parent.UserConstructionScript`))