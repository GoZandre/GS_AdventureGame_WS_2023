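; Debug interactible chest drawer, built on a parent puzzle-object class, that the player slides with the mouse; objects inside attach to it at BeginPlay.
; Tick projects the cursor at grab-point depth, offsets it by the StartInteract impact point, clamps it between two limit markers and interpolates the drawer there.
; Timelines shake it when locked and nudge it open on unlock, then switch the game instance's interaction camera.
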(event `self.ReceiveBeginPlay`
  ;[1 1 1] BaseFunction
  (`parent.ReceiveBeginPlay`)
  (set `self.BaseRelativeLocation` (`SceneComponent.RelativeLocation` (`self.ChestDrawer_Drawer`)))
  (for _array_element (`self.ObjectInside`)
    (`self.K2_AttachToComponent` _array_element (`self.ChestDrawer_Drawer`) "None" "KeepWorld" "KeepWorld" "KeepWorld" true)))

(event `self.VerifyCondition`
  ;[1 1 1] BaseFunction
  (`parent.VerifyCondition`))

(event `self.PuzzleSolved`
  ;[1 1 1] BaseFunction
  (`parent.PuzzleSolved`)
  (`KismetSystemLibrary.PrintString` "Win"))

(event `self.PuzzleUnsloved`
  ;[1 1 1] BaseFunction
  (`parent.PuzzleUnsloved`))

(event `self.CantInteractFeedback`
  (bind _baserelativelocation (`self.BaseRelativeLocation`))
  (`TimelineComponent.SetPlayRate` (`self.LockedLerp`) 2.0)
  (bind (_direction _lerpshake) (`Timeline|LockedLerp` :!via `PlayFromStart`)
    (:`Update`
      (`SceneComponent.K2_SetRelativeLocation` (`self.ChestDrawer_Drawer`) (`KismetMathLibrary.VLerp` _baserelativelocation (+ _baserelativelocation (`KismetMathLibrary.MakeVector` 1.0)) _lerpshake) false false))))

(event `/Game/BlueprintActors/InteractibleObjects/BPI_Interact.StartInteract`
  (params (ImpactLocation :type "Vector Structure"))
  ;[1 1 1] BaseFunction
  (set `self.Impact LocationDifference` (- ImpactLocation (`SceneComponent.K2_GetComponentLocation` (`self.ChestDrawer_Drawer`))))
  (`parent.StartInteract` ImpactLocation))

(event `/Game/BlueprintActors/InteractibleObjects/BPI_Interact.UnlockInteract`
  (bind _baserelativelocation (`self.BaseRelativeLocation`))
  ;[1 1 1] BaseFunction
  (`parent.UnlockInteract`)
  (bind (_direction _unlocklerp) (`Timeline|Timeline` :!via `PlayFromStart`)
    (:`Update`
      (`SceneComponent.K2_SetRelativeLocation` (`self.ChestDrawer_Drawer`) (`KismetMathLibrary.VLerp` _baserelativelocation (+ _baserelativelocation (`KismetMathLibrary.MakeVector` 5.0)) _unlocklerp) false false))
    (:`Finished`
      (bind _asadventure_game_istance (cast `/Game/Config/GameInstance/AdventureGameIstance` (`GameplayStatics.GetGameInstance`)))
      (`/Game/Config/GameInstance/AdventureGameIstance.RemoveLastCamera` _asadventure_game_istance)
      (`/Game/Config/GameInstance/AdventureGameIstance.AddInteractionCamera` _asadventure_game_istance (`self.NewCameraOnUnlock`) "NewEnumerator2"))))

(event `self.ReceiveTick`
  (params (DeltaSeconds :type "Float (single-precision)"))
  (bind _chestdrawer_drawer (`self.ChestDrawer_Drawer`))
  (bind (_worldlocation _worlddirection) (`PlayerController.DeprojectMousePositionToWorld` (`GameplayStatics.GetPlayerController` 0)))
  (`parent.ReceiveTick` DeltaSeconds)
  (`SceneComponent.K2_SetWorldLocation` _chestdrawer_drawer (`KismetMathLibrary.VInterpTo` (`SceneComponent.K2_GetComponentLocation` _chestdrawer_drawer) (`KismetMathLibrary.FindClosestPointOnSegment` (- (+ _worldlocation (* _worlddirection (`KismetMathLibrary.VSize` (- _worldlocation (+ (`SceneComponent.K2_GetComponentLocation` _chestdrawer_drawer) (`self.Impact LocationDifference`)))))) (`self.Impact LocationDifference`)) (`SceneComponent.K2_GetComponentLocation` (`self.LimitPos_01`)) (`SceneComponent.K2_GetComponentLocation` (`self.LimitPos_02`))) DeltaSeconds 10.0) false false))

(fn `UserConstructionScript`
  (`parent.UserConstructionScript`))