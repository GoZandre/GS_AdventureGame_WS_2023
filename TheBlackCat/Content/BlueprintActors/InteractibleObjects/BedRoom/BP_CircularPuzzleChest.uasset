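; Bedroom chest interactable whose lid carries an attached puzzle and becomes rotatable by mouse once unlocked.
; UnlockInteract swaps the interaction camera through AdventureGameIstance, swings the lid with a slowed timeline, then enables interaction.
; StartInteract records a base rotation, and Tick eases the lid toward the deprojected mouse angle, clamped to a quarter turn and grid-snapped.
; Puzzle condition and result events defer to the parent, with only a debug "Win" print on solve.
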(event `self.ReceiveBeginPlay`
  ;[1 1 1] BaseFunction
  (`parent.ReceiveBeginPlay`)
  (`self.K2_AttachToComponent` (`self.AttachedPuzzle`) (`self.SM_ChestPuzzleTop`) "None" "KeepWorld" "KeepWorld" "KeepWorld" true)
  (set `self.BaseRelativeLocation` (`SceneComponent.RelativeRotation` (`self.SM_ChestPuzzleTop`)))
  (`TimelineComponent.SetPlayRate` (`self.SemiOpenTimeline`) 0.25))

(event `/Game/BlueprintActors/InteractibleObjects/BPI_Interact.UnlockInteract`
  (params (ImpactLocation :type "Vector Structure"))
  (bind _baserelativelocation (`self.BaseRelativeLocation`))
  ;[1 1 1] BaseFunction
  (bind _asadventure_game_istance (cast `/Game/Config/GameInstance/AdventureGameIstance` (`GameplayStatics.GetGameInstance`)))
  (`/Game/Config/GameInstance/AdventureGameIstance.RemoveLastCamera` _asadventure_game_istance)
  (`/Game/Config/GameInstance/AdventureGameIstance.AddInteractionCamera` _asadventure_game_istance (`self.NewCameraOnUnlock`) "NewEnumerator2")
  (bind (_direction _unlocklerp) (`Timeline|SemiOpenTimeline` :!via `PlayFromStart`)
    (:`Update`
      (`SceneComponent.K2_SetRelativeRotation` (`self.SM_ChestPuzzleTop`) (`KismetMathLibrary.RLerp` _baserelativelocation (`KismetMathLibrary.MakeRotator` -90.0 (.pitch _baserelativelocation) (.yaw _baserelativelocation)) _unlocklerp) false false))
    (:`Finished`
      (set `self.CanInteract` true))))

(event `self.VerifyCondition`
  ;[1 1 1] BaseFunction
  (`parent.VerifyCondition`))

(event `self.PuzzleSolved`
  ;[1 1 1] BaseFunction
  (`parent.PuzzleSolved`)
  (`KismetSystemLibrary.PrintString` "Win"))

(event `self.PuzzleUnsloved`
  ;[1 1 1] BaseFunction
  (`parent.PuzzleUnsloved`))

(event `/Game/BlueprintActors/InteractibleObjects/BPI_Interact.StartInteract`
  (params (ImpactLocation :type "Vector Structure") (CollidedComponent :type "ActorComponent Object Reference"))
  ;[1 1 1] BaseFunction
  (set `self.NearestComponent` (`self.SM_ChestPuzzleTop`))
  (set `self.BaseRotator` (`self.GetBaseRotation`))
  (`parent.StartInteract` ImpactLocation CollidedComponent))

(event `self.ReceiveTick`
  (params (DeltaSeconds :type "Float (single-precision)"))
  (bind _sm_chestpuzzletop (`self.SM_ChestPuzzleTop`))
  (bind _relativerotation (`SceneComponent.RelativeRotation` _sm_chestpuzzletop))
  (`parent.ReceiveTick` DeltaSeconds)
  (`SceneComponent.K2_SetRelativeRotation` _sm_chestpuzzletop (`KismetMathLibrary.RInterpTo` _relativerotation (`KismetMathLibrary.MakeRotator` (`KismetMathLibrary.GridSnap_Float` (`KismetMathLibrary.FClamp` (- (.yaw (`KismetMathLibrary.FindLookAtRotation` (`SceneComponent.K2_GetComponentLocation` (`self.NearestComponent`)) (`self.GetMouseRot`))) (`self.BaseRotator`)) -90.0 0.0) (`self.RotationGrid`)) (.pitch _relativerotation) (.yaw _relativerotation)) DeltaSeconds 10.0) false false))

(fn `UserConstructionScript`
  (`parent.UserConstructionScript`))