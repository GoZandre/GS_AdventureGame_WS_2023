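; BP_Interupter is a debug puzzle switch whose lever pitches toward the mouse cursor.
; Every Tick, it deprojects the cursor near the lever's depth and smoothly interpolates pitch, clamped between RotationStart and RotationEnd.
; VerifyCondition combines two condition checks, whose graphs show only unconnected comparisons of pitch against a target plus or minus a margin.
; Solved and unsolved events extend parent logic by messaging AffectedObject.
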(event `self.ReceiveBeginPlay`
  ;[1 1 1] BaseFunction
  (`parent.ReceiveBeginPlay`)
  (`SceneComponent.K2_SetRelativeRotation` (`self.Interupter_01_Interupt`) (`SceneComponent.RelativeRotation` (`self.RotationStart`)) false false))

(event `self.VerifyCondition`
  ;[1 1 1] BaseFunction
  (`parent.VerifyCondition`)
  (set `self.PuzzleCompleted` (and (`self.PuzzleCondition_01`) (`self.PuzzleCondition_02`))))

(event `self.PuzzleSolved`
  ;[1 1 1] BaseFunction
  (`parent.PuzzleSolved`)
  (message `/Game/BlueprintActors/InteractibleObjects/BPI_PuzzleSolving.Solved` (`self.AffectedObject`)))

(event `self.PuzzleUnsloved`
  ;[1 1 1] BaseFunction
  (`parent.PuzzleUnsloved`)
  (message `/Game/BlueprintActors/InteractibleObjects/BPI_PuzzleSolving.Unsolved` (`self.AffectedObject`)))

(event `self.ReceiveTick`
  (params (DeltaSeconds :type "Float (single-precision)"))
  (bind _interupter_01_interupt (`self.Interupter_01_Interupt`))
  (bind (_worldlocation _worlddirection) (`PlayerController.DeprojectMousePositionToWorld` (`GameplayStatics.GetPlayerController` 0)))
  (bind _returnvalue (`SceneComponent.K2_GetComponentLocation` _interupter_01_interupt))
  (bind (_relativerotation_roll _relativerotation_pitch) (`KismetMathLibrary.BreakRotator` (`SceneComponent.RelativeRotation` (`self.RotationEnd`))))
  (bind (_relativerotation_roll_2 _relativerotation_pitch_2) (`KismetMathLibrary.BreakRotator` (`SceneComponent.RelativeRotation` (`self.RotationStart`))))
  (bind (_returnvalue_roll _returnvalue_pitch) (`KismetMathLibrary.BreakRotator` (`KismetMathLibrary.FindLookAtRotation` _returnvalue (+ _worldlocation (* _worlddirection (- (`KismetMathLibrary.VSize` (- _returnvalue _worldlocation)) 10.0))))))
  ;[1 1 1] Interaction
  (`parent.ReceiveTick` DeltaSeconds)
  (`SceneComponent.K2_SetRelativeRotation` _interupter_01_interupt (`KismetMathLibrary.RInterpTo` (`SceneComponent.RelativeRotation` _interupter_01_interupt) (`KismetMathLibrary.MakeRotator` 0.0 (`KismetMathLibrary.FClamp` _returnvalue_pitch _relativerotation_pitch_2 _relativerotation_pitch)) DeltaSeconds 10.0) false false))

(fn `UserConstructionScript`
  (`parent.UserConstructionScript`))