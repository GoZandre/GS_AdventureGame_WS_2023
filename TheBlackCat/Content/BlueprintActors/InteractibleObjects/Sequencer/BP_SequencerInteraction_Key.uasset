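; A key interactible, built on a parent sequencer interaction Blueprint, that plays as a two-step interaction sequence.
; On BeginPlay it rebuilds SequenceToDo with a movement step targeting MovementLimitB, then a rotation step targeting RotationMin, each bounded by its own limits.
; UnlockInteract passes the impact location straight to StartInteract, leaving the sequence logic to inherited code.
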(event `self.ReceiveBeginPlay`
  (bind _movementlimitb (`self.MovementLimitB`))
  (bind _sequencetodo (`self.SequenceToDo`))
  (bind _rotationmin (`self.RotationMin`))
  (`parent.ReceiveBeginPlay`)
  (`KismetArrayLibrary.Array_Clear` _sequencetodo)
  (`KismetArrayLibrary.Array_Add` _sequencetodo (make `/Game/BlueprintActors/InteractibleObjects/Sequencer/S_InteractionSequence` false "NewEnumerator1" (`self.MovementLimitA`) _movementlimitb _movementlimitb))
  (`KismetArrayLibrary.Array_Add` (`self.SequenceToDo`) (make `/Game/BlueprintActors/InteractibleObjects/Sequencer/S_InteractionSequence` false "NewEnumerator2" _rotationmin (`self.RotationMax`) _rotationmin)))

(event `/Game/BlueprintActors/InteractibleObjects/BPI_Interact.UnlockInteract`
  (params (ImpactLocation :type "Vector Structure"))
  (`/Game/BlueprintActors/InteractibleObjects/BPI_Interact.StartInteract` ImpactLocation))

(fn `UserConstructionScript`
  (`parent.UserConstructionScript`))