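; BP_ExploreInteraction is a trigger actor that offers an exploration interaction while the player stands in its collision volume.
; On overlap it hands BP_PlayerCharacter the linked object, camera lock point, character position and dialog, and shows a sign at SignPlace through the main widget.
; Entering also sets CanInteract on every entry in UnlockedInteractions; leaving removes the interaction and sign and disables those entries again.
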(event `self.TriggerCollision.OnComponentBeginOverlap`
  (params (OverlappedComponent :type "PrimitiveComponent Object Reference") (OtherActor :type "Actor Object Reference") (OtherComp :type "PrimitiveComponent Object Reference") (OtherBodyIndex :type Integer) (bFromSweep :type Boolean) (SweepResult :type "HitResult Structure (by ref)"))
  (bind _asbp_player_character (cast `/Game/ThirdPerson/Blueprints/BP_PlayerCharacter` OtherActor))
  (message `/Game/BlueprintActors/InteractionManager/BPI_ExploreInteraction.CreateExploreInteraction` _asbp_player_character (`self.LinkedInteractionObject`) (`self.LinkedInteractionPoint`) (`SceneComponent.K2_GetComponentToWorld` (`self.CharacterPosition`)) (`self.DialogOnInteract`))
  (`/Game/UserInterface/W_MainWidget.CreateInteractionSign` (`/Game/ThirdPerson/Blueprints/BP_PlayerCharacter.MainWidget` _asbp_player_character) (`SceneComponent.K2_GetComponentLocation` (`self.SignPlace`)))
  (for _array_element (`self.UnlockedInteractions`)
    (set `/Game/BlueprintActors/InteractibleObjects/BP_Interactible.CanInteract` true _array_element)))

(event `self.TriggerCollision.OnComponentEndOverlap`
  (params (OverlappedComponent :type "PrimitiveComponent Object Reference") (OtherActor :type "Actor Object Reference") (OtherComp :type "PrimitiveComponent Object Reference") (OtherBodyIndex :type Integer))
  (bind _asbp_player_character (cast `/Game/ThirdPerson/Blueprints/BP_PlayerCharacter` OtherActor))
  (`/Game/BlueprintActors/InteractionManager/BPI_ExploreInteraction.DestroyInteraction` _asbp_player_character)
  (`/Game/UserInterface/W_MainWidget.DestroyInteractionSign` (`/Game/ThirdPerson/Blueprints/BP_PlayerCharacter.MainWidget` _asbp_player_character) false)
  (for _array_element (`self.UnlockedInteractions`)
    (set `/Game/BlueprintActors/InteractibleObjects/BP_Interactible.CanInteract` false _array_element)))

(fn `UserConstructionScript`)