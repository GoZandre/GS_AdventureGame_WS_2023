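; BP_InteractionCameraPoint is a possessable camera point for interactions, letting the player look around within set limits.
; On possession by the first player controller it shows the mouse cursor, and the Back input tells the AdventureGameIstance to leave the interaction camera.
; Move input sets a target offset scaled by MaxLookAround, which Tick interpolates onto CameraView's relative rotation, returning to center at ten times the speed on release.
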(event `self.ReceiveBeginPlay`
  (add `Controller.OnPossessedPawnChanged` (`GameplayStatics.GetPlayerController` 0) (delegate `OnPossessedPawnChanged_Event`))
  (bind _asadventure_game_istance (cast `/Game/Config/GameInstance/AdventureGameIstance` (`GameplayStatics.GetGameInstance`)))
  (set `self.As Adventure Game Istance` _asadventure_game_istance))

(event `OnPossessedPawnChanged_Event`
  (params (OldPawn :type "Pawn Object Reference") (NewPawn :type "Pawn Object Reference"))
  (if (== NewPawn self)
    (set `PlayerController.bShowMouseCursor` true (`GameplayStatics.GetPlayerController` 0))))

(event `EnhancedInput|/Game/Config/Input/Actions/IA_Back`
  (params (ActionValue :type Boolean) (ElapsedSeconds :type "Float (double-precision)") (TriggeredSeconds :type "Float (double-precision)") (InputAction :type "InputAction Object Reference" :default "/Game/Config/Input/Actions/IA_Back.IA_Back"))
  (:`Triggered`
    (`/Game/Config/GameInstance/AdventureGameIstance.BackInteractionCamera` (`self.As Adventure Game Istance`))))

(event `EnhancedInput|/Game/Config/Input/Actions/IA_Move`
  (params (ActionValue :type "Vector2D Structure") (ElapsedSeconds :type "Float (double-precision)") (TriggeredSeconds :type "Float (double-precision)") (InputAction :type "InputAction Object Reference" :default "/Game/Config/Input/Actions/IA_Move.IA_Move"))
  (bind (_x _y) (`KismetMathLibrary.BreakVector2D` (`self.MaxLookAround`)))
  ;[1 1 1] Look Around
  (:`Triggered`
    (set `self.LookingValues` (`KismetMathLibrary.MakeVector2D` (* ActionValue_X _x) (* ActionValue_Y _y))))
  (:`Started`
    (set `self.ControlledLerpSpeed` (`self.LerpSpeed`)))
  (:`Completed`
    (set `self.LookingValues` (0.0 0.0))
    (set `self.ControlledLerpSpeed` (* (`self.LerpSpeed`) 10.0))))

(event `self.ReceiveTick`
  (params (DeltaSeconds :type "Float (single-precision)"))
  (bind _cameraview (`self.CameraView`))
  (bind (_x _y) (`KismetMathLibrary.BreakVector2D` (`self.LookingValues`)))
  ;[1 1 1] Look Around
  (`SceneComponent.K2_SetRelativeRotation` _cameraview (`KismetMathLibrary.RInterpTo` (`SceneComponent.RelativeRotation` _cameraview) (`KismetMathLibrary.MakeRotator` 0.0 _y _x) DeltaSeconds (`self.ControlledLerpSpeed`)) false false))

(fn `UserConstructionScript`)