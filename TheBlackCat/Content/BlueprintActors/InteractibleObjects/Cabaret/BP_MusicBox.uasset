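; Interactible music box puzzle for the cabaret, unlocked in three parts: opening the box, placing the dancer and placing the handle.
; UnlockInteract maps an index to each step and sets its flag; once all three are set, it only prints a win message.
; Opening chains lock and lid timelines, switching the interaction camera through the game instance between them.
; Dancer and handle are static mesh components added at runtime, snapped to placeholder components.
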(event `self.ReceiveBeginPlay`
  ;[1 1 1] Init Functions
  (`parent.ReceiveBeginPlay`)
  (bind _asadventure_game_istance (cast `/Game/Config/GameInstance/AdventureGameIstance` (`GameplayStatics.GetGameInstance`)))
  (set `self.As Adventure Game Istance` _asadventure_game_istance)
  (`TimelineComponent.SetPlayRate` (`self.MusicBoxOpening`) 0.5))

(event `self.VerifyCondition`
  ;[1 1 1] Init Functions
  (`parent.VerifyCondition`))

(event `self.PuzzleSolved`
  ;[1 1 1] Init Functions
  (`parent.PuzzleSolved`))

(event `self.PuzzleUnsloved`
  ;[1 1 1] Init Functions
  (`parent.PuzzleUnsloved`))

(event `/Game/BlueprintActors/InteractibleObjects/BPI_Interact.UnlockInteract`
  (params (ImpactLocation :type "Vector Structure") (UnlockIndex :type Integer))
  ;[1 1 1] Init Functions
  (`|ExecutionSequence`
    (:`then_0`
      (switch `int` UnlockIndex
        (:`0`
          (`self.OpenMusicBox`)
          (set `self.IsOpen?` true))
        (:`1`
          (`self.PlaceDancer`)
          (set `self.HasDancer?` true))
        (:`2`
          (`self.PlaceHandle`)
          (set `self.HasHandle?` true))))
    (:`then_1`
      (if (and (`self.IsOpen?`) (`self.HasDancer?`) (`self.HasHandle?`))
        (`KismetSystemLibrary.PrintString` "WIN THE GAME" true true (struct :`G` 1.0 :`B` 0.045587 :`A` 1.0))))))

(event `PlaceDancer`
  (bind _dancerposition (`self.DancerPosition`))
  ;[1 1 1] Unlock steps
  (bind _returnvalue (`AddComponent|NODE_AddStaticMeshComponent-0` :`RelativeTransform` (`SceneComponent.GetRelativeTransform` _dancerposition)))
  (`SceneComponent.K2_AttachToComponent` _returnvalue _dancerposition "None" "SnapToTarget" "SnapToTarget" "SnapToTarget" true))

(event `OpenMusicBox`
  (bind _as_adventure_game_istance (`self.As Adventure Game Istance`))
  (bind _sm_musicbox__top (`self.SM_MusicBox__Top`))
  ;[1 1 1] Unlock steps
  (bind (_direction _lerp) (`Timeline|LockerOff` :!via `PlayFromStart`)
    (:`Update`
      (`SceneComponent.K2_SetRelativeRotation` (`self.SM_MusicBox__Lock`) (`KismetMathLibrary.RLerp` (struct :`Roll` -180.0) (struct :`Roll` -10.0) _lerp) false false))
    (:`Finished`
      (`KismetSystemLibrary.Delay` 0.2)
      (`/Game/Config/GameInstance/AdventureGameIstance.RemoveLastCamera` _as_adventure_game_istance)
      (`/Game/Config/GameInstance/AdventureGameIstance.AddInteractionCamera` _as_adventure_game_istance (`self.NewCameraOnUnlock`) "NewEnumerator2")
      (bind (_direction_2 _lerp_2) (`Timeline|MusicBoxOpening` :!via `PlayFromStart`)
        (:`Update`
          (`SceneComponent.K2_SetRelativeRotation` _sm_musicbox__top (`KismetMathLibrary.RLerp` (`SceneComponent.RelativeRotation` _sm_musicbox__top) (struct :`Roll` -110.0) _lerp_2) false false))))))

(event `PlaceHandle`
  (bind _handleposition (`self.HandlePosition`))
  ;[1 1 1] Unlock steps
  (bind _returnvalue (`AddComponent|NODE_AddStaticMeshComponent-1` :`RelativeTransform` (`SceneComponent.GetRelativeTransform` _handleposition)))
  (`SceneComponent.K2_AttachToComponent` _returnvalue _handleposition "None" "SnapToTarget" "SnapToTarget" "SnapToTarget" true))

(fn `UserConstructionScript`
  (`parent.UserConstructionScript`))