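; Interactible puzzle rail, a child of a base class, whose support slides along a line between two limit points following the mouse.
; On interact it stores the grab offset; Tick projects the cursor ray at the support's depth, snaps to grid, clamps to the segment and interpolates there.
; BeginPlay attaches listed actors to CatSpawn, and unlocking spawns a cat figure puzzle there.
; Solving only adds a debug "Win" print to parent behaviour.
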(event `self.ReceiveBeginPlay`
  ;[1 1 1] BaseFunction
  (`parent.ReceiveBeginPlay`)
  (for _array_element (`self.AttachedActors`)
    (`self.K2_AttachToComponent` _array_element (`self.CatSpawn`) "None" "KeepWorld" "KeepWorld" "KeepWorld" true)))

(event `self.VerifyCondition`
  ;[1 1 1] BaseFunction
  (`parent.VerifyCondition`))

(event `self.PuzzleSolved`
  ;[1 1 1] BaseFunction
  (`parent.PuzzleSolved`)
  (`KismetSystemLibrary.PrintString` "Win"))

(event `self.PuzzleUnsloved`
  ;[1 1 1] BaseFunction
  (`parent.PuzzleUnsloved`))

(event `/Game/BlueprintActors/InteractibleObjects/BPI_Interact.StartInteract`
  (params (ImpactLocation :type "Vector Structure") (CollidedComponent :type "ActorComponent Object Reference"))
  ;[1 1 1] BaseFunction
  (set `self.Impact LocationDifference` (- ImpactLocation (`SceneComponent.K2_GetComponentLocation` (`self.Rails_01_Support`))))
  (`parent.StartInteract` ImpactLocation null))

(event `/Game/BlueprintActors/InteractibleObjects/BPI_Interact.UnlockInteract`
  (params (ImpactLocation :type "Vector Structure"))
  (bind _catspawn (`self.CatSpawn`))
  ;[1 1 1] BaseFunction
  (bind _returnvalue (`|SpawnActorFromClass` "/Game/BlueprintActors/InteractibleObjects/Entrance/BP_CatFigurePuzzle.BP_CatFigurePuzzle_C" (`SceneComponent.K2_GetComponentToWorld` _catspawn) "Undefined" "OverrideRootScale" null null))
  (`self.K2_AttachToComponent` _returnvalue _catspawn "None" "SnapToTarget" "SnapToTarget" "SnapToTarget" true))

(event `self.ReceiveTick`
  (params (DeltaSeconds :type "Float (single-precision)"))
  (bind _rails_01_support (`self.Rails_01_Support`))
  (bind (_worldlocation _worlddirection) (`PlayerController.DeprojectMousePositionToWorld` (`GameplayStatics.GetPlayerController` 0)))
  (`parent.ReceiveTick` DeltaSeconds)
  (`SceneComponent.K2_SetWorldLocation` _rails_01_support (`KismetMathLibrary.VInterpTo` (`SceneComponent.K2_GetComponentLocation` _rails_01_support) (`KismetMathLibrary.FindClosestPointOnSegment` (`KismetMathLibrary.Vector_SnappedToGrid` (- (+ _worldlocation (* _worlddirection (`KismetMathLibrary.VSize` (- _worldlocation (+ (`SceneComponent.K2_GetComponentLocation` _rails_01_support) (`self.Impact LocationDifference`)))))) (`self.Impact LocationDifference`)) 5.0) (`SceneComponent.K2_GetComponentLocation` (`self.LimitPos_02`)) (`SceneComponent.K2_GetComponentLocation` (`self.LimitPos_01`))) DeltaSeconds 10.0) false false))

(fn `UserConstructionScript`
  (`parent.UserConstructionScript`))