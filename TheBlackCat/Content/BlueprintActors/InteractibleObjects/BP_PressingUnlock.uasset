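; BP_PressingUnlock is an interactible object that unlocks other components when pressed.
; On StartInteract it walks the UnlockComponents map and calls UnlockInteract on each key, passing the impact location and that entry's value as the unlock index.
; A disconnected branch that would mark the puzzle solved and destroy the actor when DestroySelf is set never runs.
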(event `/Game/BlueprintActors/InteractibleObjects/BPI_Interact.StartInteract`
  (params (ImpactLocation :type "Vector Structure") (CollidedComponent :type "ActorComponent Object Reference"))
  (bind _unlockcomponents (`self.UnlockComponents`))
  (bind _keys (`BlueprintMapLibrary.Map_Keys` _unlockcomponents))
  (for (_array_element _array_index) _keys
    (bind _values (`BlueprintMapLibrary.Map_Values` _unlockcomponents))
    (`/Game/BlueprintActors/InteractibleObjects/BPI_Interact.UnlockInteract` _array_element ImpactLocation (`|GetArrayItem` _values _array_index))))

(fn `UserConstructionScript`
  (`parent.UserConstructionScript`))