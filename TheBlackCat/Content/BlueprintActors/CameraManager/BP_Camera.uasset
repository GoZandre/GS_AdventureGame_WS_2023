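; BP_Camera is a placeable camera actor that can serve as the player's starting view and turn to follow the character.
; On BeginPlay a start camera sends SwitchCameraMessage to the player character, while other cameras disable their tick.
; When following is enabled, Tick smoothly rotates the stationary camera toward the character's location plus an X/Y offset, with the interpolation speed set by a camera lag parameter.
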(event `self.ReceiveBeginPlay`
  (bind _returnvalue (`GameplayStatics.GetPlayerCharacter` 0))
  ;[1 1 1] Start Setup
  (if (`self.StartCamera`)
    (message `/Game/BlueprintActors/CameraManager/BPI_Camera.SwitchCamera` _returnvalue self)
    (else
      (`self.SetActorTickEnabled` false)))
  (bind _asbp_player_character (cast `/Game/ThirdPerson/Blueprints/BP_PlayerCharacter` _returnvalue))
  (set `self.As BP Player Character` _asbp_player_character))

(event `self.ReceiveTick`
  (params (DeltaSeconds :type "Float (single-precision)"))
  (bind (_followcharacter _positionoffset _cameralag) (break `/Game/BlueprintActors/CameraManager/S_CameraParameters` (`self.Param`)))
  (bind (_returnvalue_x _returnvalue_y _returnvalue_z) (`KismetMathLibrary.BreakVector` (`self.K2_GetActorLocation` (`self.As BP Player Character`))))
  (bind (_x _y) (`KismetMathLibrary.BreakVector2D` _positionoffset))
  (if _followcharacter
    (`self.K2_SetActorRotation` (`KismetMathLibrary.RInterpTo` (`self.K2_GetActorRotation`) (`KismetMathLibrary.FindLookAtRotation` (`self.K2_GetActorLocation`) (`KismetMathLibrary.MakeVector` (+ _x _returnvalue_x) (+ _y _returnvalue_y) _returnvalue_z)) DeltaSeconds _cameralag))))

(fn `UserConstructionScript`)