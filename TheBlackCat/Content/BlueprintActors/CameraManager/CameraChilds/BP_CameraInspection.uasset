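; BP_CameraInspection is a child camera for inspecting objects up close with a software-driven mouse cursor.
; Move input offsets the cursor by a sensitivity factor, and Grab traces under it to start interaction on "Interact"-tagged components, ending it on release via a bound event.
; A hit without that tag triggers a second trace that asks placing zones for help dialog.
; Back returns to the previous camera, gated by a delayed flag.
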(event `EnhancedInput|/Game/Config/Input/Actions/IA_MoveCursor`
  (params (ActionValue :type "Vector2D Structure") (ElapsedSeconds :type "Float (double-precision)") (TriggeredSeconds :type "Float (double-precision)") (InputAction :type "InputAction Object Reference" :default "/Game/Config/Input/Actions/IA_MoveCursor.IA_MoveCursor"))
  (bind _returnvalue (`GameplayStatics.GetPlayerController` 0))
  (bind _cursorsensibility (`self.CursorSensibility`))
  (bind (_locationx _locationy) (`PlayerController.GetMousePosition` _returnvalue))
  (:`Triggered`
    (`PlayerController.SetMouseLocation` _returnvalue (`KismetMathLibrary.FTrunc` (+ _locationx (* ActionValue_X _cursorsensibility))) (`KismetMathLibrary.FTrunc` (+ _locationy (* ActionValue_Y _cursorsensibility -1.0))))))

(event `EnhancedInput|/Game/Config/Input/Actions/IA_Grab`
  (params (ActionValue :type Boolean) (ElapsedSeconds :type "Float (double-precision)") (TriggeredSeconds :type "Float (double-precision)") (InputAction :type "InputAction Object Reference" :default "/Game/Config/Input/Actions/IA_Grab.IA_Grab"))
  (bind (_worldlocation _worlddirection) (`PlayerController.DeprojectMousePositionToWorld` (`GameplayStatics.GetPlayerController` 0)))
  (bind (_worldlocation_2 _worlddirection_2) (`PlayerController.DeprojectMousePositionToWorld` (`GameplayStatics.GetPlayerController` 0)))
  (:`Started`
    (if (`/Game/Config/GameInstance/AdventureGameIstance.CanGrabObject` (`self.As Adventure Game Istance`))
      (bind (_outhit _returnvalue) (`KismetSystemLibrary.LineTraceSingle` :`Start` _worldlocation :`End` (+ _worldlocation (* _worlddirection 1000.0)) :`TraceChannel` "TraceTypeQuery1" :`DrawTime` 10.0))
      (if _returnvalue
        (bind (_bblockinghit _binitialoverlap _time _distance _location _impactpoint _normal _impactnormal _physmat _hitactor _hitcomponent) (`GameplayStatics.BreakHitResult` _outhit))
        (if (`ActorComponent.ComponentHasTag` _hitcomponent "Interact")
          (add `self.ObjectGrabed` (delegate `StopGrabbing`))
          (message `/Game/BlueprintActors/InteractibleObjects/BPI_Interact.StartInteract` _hitactor _impactpoint _hitcomponent)
          (else
            (bind (_outhit_2 _returnvalue_2) (`KismetSystemLibrary.LineTraceSingle` :`Start` _worldlocation_2 :`End` (+ _worldlocation_2 (* _worlddirection_2 1000.0)) :`TraceChannel` "TraceTypeQuery4" :`DrawTime` 10.0))
            (if _returnvalue_2
              (bind _asbp_object_placing_zone (cast `/Game/BlueprintActors/InteractibleObjects/BP_ObjectPlacingZone` (`.HitActor` (`GameplayStatics.BreakHitResult` _outhit_2))))
              (`/Game/BlueprintActors/InteractibleObjects/BP_ObjectPlacingZone.CallHelpDialog` _asbp_object_placing_zone)))))))
  (:`Canceled`
    (`self.ObjectGrabed` :!label _label))
  (:`Completed`
    (goto _label)))

(event `StopGrabbing`
  (message `/Game/BlueprintActors/InteractibleObjects/BPI_Interact.EndInteract` (`.HitActor` (`GameplayStatics.BreakHitResult` (stale `EnhancedInput|/Game/Config/Input/Actions/IA_Grab` _outhit)))))

(event `EnhancedInput|/Game/Config/Input/Actions/IA_Back`
  (params (ActionValue :type Boolean) (ElapsedSeconds :type "Float (double-precision)") (TriggeredSeconds :type "Float (double-precision)") (InputAction :type "InputAction Object Reference" :default "/Game/Config/Input/Actions/IA_Back.IA_Back"))
  (:`Started`
    (if (`self.CanBackCamera`)
      (set `PlayerController.bShowMouseCursor` true (`GameplayStatics.GetPlayerController` 0))
      (`/Game/Config/GameInstance/AdventureGameIstance.BackInteractionCamera` (`self.As Adventure Game Istance`) (`self.CameraBackTransition`))
      (else
        (`KismetSystemLibrary.Delay` 1.0)
        (set `self.CanBackCamera` true)))))

(fn `UserConstructionScript`
  (`parent.UserConstructionScript`))