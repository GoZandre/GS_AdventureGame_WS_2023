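; Interactible puzzle actor where the player drags a linked item through ordered move and rotate steps using the mouse.
; The first interaction spawns the item mesh, and later ones bind step advancement to the FollowSequence dispatcher.
; Tick eases the item toward the deprojected cursor, constrained to a segment or clamped X rotation, firing FollowSequence near the objective.
; The last step unlocks linked interactions, reports the puzzle solved and destroys the actor.
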(event `self.ReceiveBeginPlay`
  (`parent.ReceiveBeginPlay`)
  (set `self.CanInteract` false))

(event `self.StartInteract`
  (params (ImpactLocation :type "Vector Structure") (CollidedComponent :type "ActorComponent Object Reference"))
  (bind _itemstartposition (`self.ItemStartPosition`))
  ;[1 1 1] Setup
  (`parent.StartInteract` ImpactLocation null)
  (if (`self.CanInteract`)
    (set `self.Impact LocationDifference` (- ImpactLocation (`SceneComponent.K2_GetComponentLocation` (`self.ItemStartPosition`))))
    (add `self.FollowSequence` (delegate `NextSequence`))
    (else
      (set `self.CanInteract` true)
      (bind _returnvalue (`AddComponent|NODE_AddStaticMeshComponent-0` :`RelativeTransform` (`SceneComponent.K2_GetComponentToWorld` _itemstartposition)))
      (`SceneComponent.K2_AttachToComponent` _returnvalue _itemstartposition "None" "SnapToTarget" "SnapToTarget" "SnapToTarget" true)
      (`StaticMeshComponent.SetStaticMesh` _returnvalue (`self.LinkedItem`))
      (set `ActorComponent.ComponentTags` (`|MakeArray` "Interact" :!type "Name") _returnvalue))))

(event `self.ReceiveTick`
  (params (DeltaSeconds :type "Float (single-precision)"))
  (bind _sequencetodo (`self.SequenceToDo`))
  (bind _currentindexsequence (`self.CurrentIndexSequence`))
  (bind (_iscompleted _interactiontype _limita _limitb _objective _clampedrotation) (break `/Game/BlueprintActors/InteractibleObjects/Sequencer/S_InteractionSequence` (`|GetArrayItem` _sequencetodo _currentindexsequence)))
  (`parent.ReceiveTick` DeltaSeconds)
  (if (<= _currentindexsequence (- (`KismetArrayLibrary.Array_Length` _sequencetodo) 1))
    (switch `/Game/BlueprintActors/InteractibleObjects/Sequencer/E_InteractionSequenceType` _interactiontype
      (:`NewEnumerator1`
        (`self.MovingSequence` (`SceneComponent.K2_GetComponentLocation` _limita) (`SceneComponent.K2_GetComponentLocation` _limitb) (`SceneComponent.K2_GetComponentLocation` _objective)))
      (:`NewEnumerator2`
        (`self.RotatingSequence` (`SceneComponent.RelativeRotation` _limita) (`SceneComponent.RelativeRotation` _limitb) (`SceneComponent.RelativeRotation` _objective) _clampedrotation)))))

(event `NextSequence`
  (remove `self.FollowSequence` (delegate `NextSequence`))
  (if (< (`self.CurrentIndexSequence`) (- (`KismetArrayLibrary.Array_Length` (`self.SequenceToDo`)) 1))
    (`/Engine/EditorBlueprintResources/StandardMacros.IncrementInt` (`self.CurrentIndexSequence`)
      (:`  `
        (`self.EndInteract`)))
    (else
      (for _array_element (`self.InteractionOnComplete`)
        (`self.UnlockInteract` _array_element (0.0 0.0 0.0))
        (message `/Game/Config/SaveSystem/BPI_SaveConfiguration.AddUnlockedElement` (`GameplayStatics.GetGameInstance`) _array_element))
      (`self.PuzzleSolved`)
      (`self.K2_DestroyActor`))))

(event `MovingSequence`
  (params (LimitA :type "Vector Structure") (LimitB :type "Vector Structure") (Objective :type "Vector Structure"))
  (bind _itemstartposition (`self.ItemStartPosition`))
  (`SceneComponent.K2_SetWorldLocation` _itemstartposition (`KismetMathLibrary.VInterpTo` (`SceneComponent.K2_GetComponentLocation` _itemstartposition) (`KismetMathLibrary.FindClosestPointOnSegment` (`self.GetMousePos`) LimitA LimitB) (`GameplayStatics.GetWorldDeltaSeconds`) 10.0) false false)
  ;[1 1 1] VerifyCondition
  (if (== (`SceneComponent.K2_GetComponentLocation` (`self.ItemStartPosition`)) Objective :`ErrorTolerance` (`self.MarginOfError`))
    (`self.FollowSequence`)))

(event `RotatingSequence`
  (params (LimitA :type "Rotator Structure") (LimitB :type "Rotator Structure") (Objective :type "Rotator Structure") (ClampedAxis :type "EMotionExtractor_Axis Enum" :default "X"))
  (bind _itemstartposition (`self.ItemStartPosition`))
  (bind _relativerotation (`SceneComponent.RelativeRotation` _itemstartposition))
  (bind _relativerotation_2 (`SceneComponent.RelativeRotation` (`self.ItemStartPosition`)))
  (switch `EMotionExtractor_Axis` ClampedAxis
    (:`X`
      (`SceneComponent.K2_SetRelativeRotation` _itemstartposition (`KismetMathLibrary.RInterpTo` _relativerotation (`KismetMathLibrary.MakeRotator` (`KismetMathLibrary.FClamp` (.roll (`KismetMathLibrary.MakeRotFromZY` (`self.GetMouseRot`) (`SceneComponent.K2_GetComponentLocation` (`self.ItemStartPosition`)))) (.roll LimitA) (.roll LimitB)) (.pitch _relativerotation) (.yaw _relativerotation)) (`GameplayStatics.GetWorldDeltaSeconds`) 10.0) false false)
      ;[1 1 1] VerifyCondition
      (if (== _relativerotation_2 (`KismetMathLibrary.MakeRotator` (.roll Objective) (.pitch _relativerotation_2) (.yaw _relativerotation_2)) :`ErrorTolerance` (`self.MarginOfError`))
        (`self.FollowSequence`)))))

(fn `UserConstructionScript`
  (`parent.UserConstructionScript`))