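; BP_CameraPoint is a possessable camera viewpoint for examining interactive spots and placing inventory items on them.
; On possession it shows the cursor, and rotation input eases the view within set limits, returning faster on release.
; While an item moves, a cursor trace finds BP_ObjectPlacingZone actors and updates the preview by ID match.
; A valid placement disables backing out, sends the zone's unlock message and removes the item through the game instance.
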(event `EnhancedInput|/Game/Config/Input/Actions/IA_Inventory`
  (params (ActionValue :type Boolean) (ElapsedSeconds :type "Float (double-precision)") (TriggeredSeconds :type "Float (double-precision)") (InputAction :type "InputAction Object Reference" :default "/Game/Config/Input/Actions/IA_Inventory.IA_Inventory"))
  (:`Triggered`
    (message `/Game/Config/Inventory/BPI_InventoryInterface.CallInventory` (`GameplayStatics.GetGameInstance`))))

(event `self.ReceiveBeginPlay`
  (add `Controller.OnPossessedPawnChanged` (`GameplayStatics.GetPlayerController` 0) (delegate `OnPossessedPawnChanged_Event`))
  (bind _asadventure_game_istance (cast `/Game/Config/GameInstance/AdventureGameIstance` (`GameplayStatics.GetGameInstance`)))
  (set `self.As Adventure Game Istance` _asadventure_game_istance))

(event `OnPossessedPawnChanged_Event`
  (params (OldPawn :type "Pawn Object Reference") (NewPawn :type "Pawn Object Reference"))
  (if (== NewPawn self)
    (set `PlayerController.bShowMouseCursor` true (`GameplayStatics.GetPlayerController` 0))
    (`self.OnPossess`)))

(event `OnPossess`
  (set `self.CanBackCamera` true))

(event `EnhancedInput|/Game/Config/Input/Actions/IA_RotateCamera`
  (params (ActionValue :type "Vector2D Structure") (ElapsedSeconds :type "Float (double-precision)") (TriggeredSeconds :type "Float (double-precision)") (InputAction :type "InputAction Object Reference" :default "/Game/Config/Input/Actions/IA_RotateCamera.IA_RotateCamera"))
  (bind (_x _y) (`KismetMathLibrary.BreakVector2D` (`self.MaxLookAround`)))
  ;[1 1 1] Look Around
  (:`Triggered`
    (set `self.LookingValues` (`KismetMathLibrary.MakeVector2D` (* ActionValue_X _x) (* ActionValue_Y _y -1.0))))
  (:`Started`
    (set `self.ControlledLerpSpeed` (`self.LerpSpeed`)))
  (:`Canceled`
    (set `self.LookingValues` (0.0 0.0) :!label _label)
    (set `self.ControlledLerpSpeed` (* (`self.LerpSpeed`) 10.0)))
  (:`Completed`
    (goto _label)))

(event `self.ReceiveTick`
  (params (DeltaSeconds :type "Float (single-precision)"))
  ;[1 1 1] Look Around
  (`self.CameraLookingMovement` DeltaSeconds)
  (`self.MovingItem`))

(event `TakeItemFromInventory`
  (params (TakedItem :type "/Game/Config/Inventory/S_Item Structure") (ItemPreviewWidget :type "/Game/UserInterface/W_ItemPlacementPreview Object Reference"))
  ;[0.1771 0.1771 0.1771] Items Placement
  (set `self.Taked Item` TakedItem)
  (set `self.Item Preview Widget` ItemPreviewWidget)
  (add `self.PlacingItem` (delegate `Event_VerifyItemPlacement`))
  (add `self.MovingItem` (delegate `Event_ItemMove`)))

(event `Event_ItemMove`
  (bind _returnvalue (`WidgetLayoutLibrary.GetViewportScale`))
  (bind _item_preview_widget (`self.Item Preview Widget`))
  ;[0.1771 0.1771 0.1771] Items Placement
  (bind _returnvalue_2 (`WidgetLayoutLibrary.GetMousePositionOnViewport`))
  (bind (_worldposition _worlddirection) (`GameplayStatics.DeprojectScreenToWorld` (`GameplayStatics.GetPlayerController` 0) (* _returnvalue_2 (`KismetMathLibrary.MakeVector2D` _returnvalue _returnvalue))))
  (bind (_outhit _returnvalue_3) (`KismetSystemLibrary.LineTraceSingle` _worldposition (+ _worldposition (* _worlddirection 100.0)) "TraceTypeQuery4"))
  (if _returnvalue_3
    (bind _asbp_object_placing_zone (cast `/Game/BlueprintActors/InteractibleObjects/BP_ObjectPlacingZone` (`.HitActor` (`GameplayStatics.BreakHitResult` _outhit))))
    (if (`/Game/BlueprintActors/InteractibleObjects/BP_Interactible.CanInteract` _asbp_object_placing_zone)
      (bind _same (`/Game/BlueprintActors/InteractibleObjects/BP_ObjectPlacingZone.HasRightID` _asbp_object_placing_zone (`.ID_11_22A84D6745929FB27C0D0B96CECC51E9` (break `/Game/Config/Inventory/S_Item` (`self.Taked Item`)))))
      (if _same
        (message `/Game/UserInterface/WidgetInterface/BPI_ItemPlacingPreviewValidation.ValidPreview` _item_preview_widget)
        (set `self.As BP Object Placing Zone` _asbp_object_placing_zone)
        (else
          (message `/Game/UserInterface/WidgetInterface/BPI_ItemPlacingPreviewValidation.UnvalidPreview` _item_preview_widget :!label _label_2)
          (set `self.As BP Object Placing Zone` null))))
    (else
      (goto _label_2))))

(event `Event_VerifyItemPlacement`
  (bind _as_bp_object_placing_zone (`self.As BP Object Placing Zone`))
  ;[0.1771 0.1771 0.1771] Items Placement
  (`|ExecutionSequence`
    (:`then_0`
      (remove `self.MovingItem` (delegate `Event_ItemMove`)))
    (:`then_1`
      (if (!= null _as_bp_object_placing_zone)
        (set `self.CanBackCamera` false)
        (message `/Game/BlueprintActors/InteractibleObjects/BPI_Interact.UnlockInteract` (`/Game/BlueprintActors/InteractibleObjects/BP_ObjectPlacingZone.UnlockOnCombine` _as_bp_object_placing_zone) (0.0 0.0 0.0) (`/Game/BlueprintActors/InteractibleObjects/BP_ObjectPlacingZone.UnlockIndex` _as_bp_object_placing_zone))
        (message `/Game/Config/Inventory/BPI_ItemsInteraction.RemoveItemFromInventory` (`self.As Adventure Game Istance`) (`self.Taked Item`))))))

(event `EnhancedInput|/Game/Config/Input/Actions/IA_Menu`
  (params (ActionValue :type Boolean) (ElapsedSeconds :type "Float (double-precision)") (TriggeredSeconds :type "Float (double-precision)") (InputAction :type "InputAction Object Reference" :default "/Game/Config/Input/Actions/IA_Menu.IA_Menu"))
  (:`Triggered`
    (`/Game/UserInterface/W_MainWidget.PauseGame` (`/Game/ThirdPerson/Blueprints/BP_PlayerCharacter.MainWidget` (`/Game/Config/GameInstance/AdventureGameIstance.PlayerCharacter` (`self.As Adventure Game Istance`))))))

(fn `CameraLookingMovement`
  (params (DeltaSeconds :type "Float (single-precision)"))
  (bind _cameraview (`self.CameraView`))
  (bind (_x _y) (`KismetMathLibrary.BreakVector2D` (`self.LookingValues`)))
  (`SceneComponent.K2_SetRelativeRotation` _cameraview (`KismetMathLibrary.RInterpTo` (`SceneComponent.RelativeRotation` _cameraview) (`KismetMathLibrary.MakeRotator` 0.0 _y _x) DeltaSeconds (`self.ControlledLerpSpeed`)) false false))

(fn `ClearRenderTexture`)

(fn `SetRenderTexture`)

(fn `UserConstructionScript`)